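; BP_Tank is the player-controlled tank, handling driving, aiming, firing and opening the pause menu.
; Axis inputs move the actor along local X, yaw the controller, and rotate StaticMesh4 and Socket separately for aiming.
; Releasing Primary Action spawns BP_Bullet, sound and an emitter at every StaticMesh8 socket, gated by CanFire and a FireDelay cooldown.
; P shows a cached UI_Pause widget, switches to UI-only input and pauses the game.
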(event EventBeginPlay
  (Input|SetInputModeGameOnly (Game|GetPlayerController 0)))

(event Input|ActionEvents|InputActionPrimaryAction
  (params (Key :type Key%20Structure :default "None"))
  (bind _staticmesh8 (Variables|Default|GetStaticMesh8))
  (:Released
    (if (Variables|Default|GetCanFire)
      (for _array_element (Transformation|GetAllSocketNames _staticmesh8)
        (Variables|Default|SetCanFire false)
        (Game|SpawnActorfromClass "/Game/Blueprints/BP_Bullet.BP_Bullet_C" (Transformation|GetSocketTransform _staticmesh8 _array_element "RTS_World") "Undefined" 0 0)
        (Audio|PlaySoundatLocation "/Game/StarterContent/Audio/Explosion01.Explosion01" (.Location (Math|Transform|BreakTransform (Transformation|GetSocketTransform _staticmesh8 _array_element "RTS_World"))) "0, 0, 0" 1.0 1.0 0.0 0 0 0)
        (Effects|SpawnEmitteratLocation 0 (.Location (Math|Transform|BreakTransform (Transformation|GetSocketTransform _staticmesh8 _array_element "RTS_World"))) (.Rotation (Math|Transform|BreakTransform (Transformation|GetSocketTransform _staticmesh8 _array_element "RTS_World"))))
        (Utilities|FlowControl|Delay (Variables|Default|GetFireDelay))
        (Variables|Default|SetCanFire true)))))

(event Input|AxisEvents|InputAxisMoveX
  (params (AxisValue :type Float%20%28single-precision%29))
  (Transformation|AddActorLocalOffset (Math|Vector|MakeVector (* AxisValue (Variables|Default|GetFordwardSpeed)) 0.0 0.0) false false))

(event Input|AxisEvents|InputAxisMoveY
  (params (AxisValue :type Float%20%28single-precision%29))
  (Pawn|Input|AddControllerYawInput (* AxisValue (Variables|Default|GetTurnSpeed))))

(event Input|AxisEvents|InputAxisCameraControlX
  (params (AxisValue :type Float%20%28single-precision%29))
  (Transformation|AddLocalRotation (Variables|Default|GetStaticMesh4) (Math|Rotator|MakeRotator 0.0 0.0 (* AxisValue (Variables|Default|GetLookSpeed))) false false))

(event Input|AxisEvents|InputAxisCameraControlY
  (params (AxisValue :type Float%20%28single-precision%29))
  (Transformation|AddLocalRotation (Variables|Default|GetSocket) (Math|Rotator|MakeRotator (* AxisValue (Variables|Default|GetLookSpeedY)) 0.0 0.0) false false))

(event Input|KeyboardEvents|P
  (params (Key :type Key%20Structure :default "None"))
  (bind _returnvalue (Game|GetPlayerController 0))
  (:Pressed
    (Utilities|IsValid (Variables|Default|GetHUD%20Reference)
      (:Is%20Valid
        _)
      (:Is%20Not%20Valid
        (bind _returnvalue_2 (UserInterface|CreateWidget "/Game/Blueprints/UI_Pause.UI_Pause_C"))
        (Variables|Default|SetHUD%20Reference _returnvalue_2)))
    (Input|SetInputModeUIOnly _returnvalue (Variables|Default|GetHUD%20Reference) "DoNotLock")
    (Variables|/Script/Engine.PlayerController|SetbShowMouseCursor _returnvalue true)
    (UserInterface|Viewport|AddtoViewport (Variables|Default|GetHUD%20Reference) 0)
    (Game|SetGamePaused true)))

(fn ConstructionScript)