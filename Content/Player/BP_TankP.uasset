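; BP_TankP is a player-controlled tank driven directly by four input axis events.
; Move axes apply local offsets for forward and back travel and local yaw rotation for steering, scaled by speed variables without delta time.
; Camera axes yaw StaticMesh4, likely the turret, and rotate Socket around its roll axis, each with its own look speed.
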(event Input|AxisEvents|InputAxisMoveX
  (params (AxisValue :type Float%20%28single-precision%29))
  (Transformation|AddActorLocalOffset (Math|Vector|MakeVector (* AxisValue (Variables|Default|GetForwardSpeed)) 0.0 0.0) false false))

(event Input|AxisEvents|InputAxisMoveY
  (params (AxisValue :type Float%20%28single-precision%29))
  (Transformation|AddActorLocalRotation (Math|Rotator|MakeRotator 0.0 0.0 (* AxisValue (Variables|Default|GetTurnSpeed))) false false))

(event Input|AxisEvents|InputAxisCameraControlX
  (params (AxisValue :type Float%20%28single-precision%29))
  (Transformation|AddLocalRotation (Variables|Default|GetStaticMesh4) (Math|Rotator|MakeRotator 0.0 0.0 (* AxisValue (Variables|Default|GetLookSpeed))) false false))

(event Input|AxisEvents|InputAxisCameraControlY
  (params (AxisValue :type Float%20%28single-precision%29))
  (Transformation|AddLocalRotation (Variables|Default|GetSocket) (Math|Rotator|MakeRotator (* AxisValue (Variables|Default|GetLookSpeedY)) 0.0 0.0) false false))

(fn ConstructionScript)