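; BP_WinCon is a win-condition actor that ends the game in victory when a BP_Tank overlaps it.
; On overlap it plays a sound at the player controller's location, then calls Win on BP_HUD.
; Once that HUD call succeeds, it switches input to UI-only and opens the Main level after a short delay.
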(event Collision|EventActorBeginOverlap
  (params (OtherActor :type Actor%20Object%20Reference))
  (bind _returnvalue (Game|GetPlayerController 0))
  (Utilities|Casting|CastToBP_Tank OtherActor)
  (Audio|PlaySoundatLocation "/Game/StarterContent/Audio/Starter_Music01.Starter_Music01" (Transformation|GetActorLocation (Game|GetPlayerController 0)) "0, 0, 0" 1.0 1.0 0.0 0 0 0)
  (bind _asbp_hud (Utilities|Casting|CastToBP_HUD (HUD|GetHUD _returnvalue)))
  (Default|Win _asbp_hud)
  (Input|SetInputModeUIOnly _returnvalue 0 "DoNotLock")
  (Utilities|FlowControl|Delay 3.0)
  (Game|OpenLevel(byName) "Main"))

(fn ConstructionScript)