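; BP_Axe is an axe hazard that destroys the tank on contact and loses the game.
; On BeginPlay, the Move timeline drives the pitch of StaticMesh5, scaling its track value by the Angle variable.
; When a BP_Tank overlaps the actor, it spawns an explosion at the tank, destroys it and calls Lose on BP_HUD.
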(event EventBeginPlay
  (bind _newtrack_0 (Timeline|move Play)
    (:Update
      (Transformation|SetRelativeRotation (Variables|Default|GetStaticMesh5) (Math|Rotator|MakeRotator 0.0 (* _newtrack_0 (Variables|Default|GetAngle)) 0.0) false false))))

(event Collision|EventActorBeginOverlap
  (params (OtherActor :type Actor%20Object%20Reference))
  (bind _asbp_tank (Utilities|Casting|CastToBP_Tank OtherActor))
  (Effects|SpawnEmitteratLocation "/Game/StarterContent/Particles/P_Explosion.P_Explosion" (Transformation|GetActorLocation _asbp_tank))
  (Actor|DestroyActor _asbp_tank)
  (bind _asbp_hud (Utilities|Casting|CastToBP_HUD (HUD|GetHUD (Game|GetPlayerController 0))))
  (Default|Lose _asbp_hud))

(fn ConstructionScript)