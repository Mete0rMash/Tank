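; BP_spawner is an actor that periodically spawns short-lived BP_target actors at an offset from its own location.
; A looping timer started on BeginPlay rolls a random integer against Probability, so higher values make spawns rarer.
; Each spawned target receives MyController as its TargetController and is stored in MyTarget.
; A second timer destroys that target shortly afterwards, before the next spawn roll, if it is still valid.
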(event Custom|SpawnTarget
  (if (> (Math|Random|RandomInteger 10) (Variables|Default|Getprobability))
    (bind _returnvalue (Game|SpawnActorfromClass "/Game/Blueprints/BP_Target.BP_target_C" (Math|Transform|MakeTransform (+ (Transformation|GetActorLocation) (Variables|Default|GetpositionToAdd)) "0, 0, 0" "1,1,1") "Undefined" 0 0 0))
    (bind _output_get (Variables|Default|SetmyTarget _returnvalue))
    (Variables|/Game/Blueprints/BP_Target.BP_target_C|SettargetController _output_get (Variables|Default|GetmyController))
    (Utilities|Time|SetTimerbyFunctionName 0 "DestroyTarget" 2.0)))

(event Custom|DestroyTarget
  (if (Utilities|IsValid (Variables|Default|GetmyTarget))
    (Actor|DestroyActor (Variables|Default|GetmyTarget))))

(event EventBeginPlay
  (Utilities|Time|SetTimerbyFunctionName 0 "SpawnTarget" 3.0 true))

(fn ConstructionScript)